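; ArcGIS map actor that sets up a HUD and moves the ArcGIS pawn to a hard-coded geographic location on input.
; BeginPlay shows the HUD with UI-only input and cursor, adds the Enhanced Input mapping context, and caches the pawn's location component.
; The SpaceBar action sets the pawn's WGS84 position, then after a short delay recenters the map origin beneath it and prints the origin coordinates.
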(event `CreateUI`
  (bind _returnvalue (`GameplayStatics.GetPlayerController` 0))
  (bind _returnvalue_2 (`|CreateWidget` "/Game/Scenes/wbp_HUD.wbp_HUD_C" _returnvalue))
  (`UserWidget.AddToViewport` _returnvalue_2 0)
  (`WidgetBlueprintLibrary.SetInputMode_UIOnlyEx` _returnvalue _returnvalue_2)
  (set `PlayerController.bShowMouseCursor` true _returnvalue))

(event `self.ReceiveBeginPlay`
  (`self.CreateUI`)
  (message `EnhancedInputSubsystemInterface.AddMappingContext` (pcsubsystem `EnhancedInputLocalPlayerSubsystem` (`GameplayStatics.GetPlayerController` 0)) "/Game/Scenes/IMC_MappingContext.IMC_MappingContext" 0 (struct))
  (bind _returnvalue (`GameplayStatics.GetActorOfClass` "/Script/ArcGISSamples.ArcGISPawn"))
  (bind _output_get (set `self.ArcGISPawn` _returnvalue))
  (set `self.ArcGISLocation` (`self.GetComponentByClass` _output_get "/Script/ArcGISMapsSDK.ArcGISLocationComponent")))

(event `EnhancedInput|/Game/Scenes/IA_SpaceBar`
  (params (ActionValue :type Boolean) (ElapsedSeconds :type "Float (double-precision)") (TriggeredSeconds :type "Float (double-precision)") (InputAction :type "InputAction Object Reference" :default "/Game/Scenes/IA_SpaceBar.IA_SpaceBar"))
  (bind _returnvalue (`ArcGISMapComponent.GetOriginPosition` (`self.mapComponent`)))
  (:`Started`
    (bind _returnvalue_2 (`ArcGISSpatialReference.WGS84`))
    (bind _returnvalue_3 (`ArcGISPoint.CreateArcGISPointWithXYZSpatialReference` -117.1825 34.055 2000.0 _returnvalue_2))
    (`/Engine/EditorBlueprintResources/StandardMacros.IsValid` (`self.GetComponentByClass` (`self.ArcGISPawn`) "/Script/ArcGISMapsSDK.ArcGISLocationComponent")
      (:`Is Valid`
        (`ArcGISLocationComponent.SetPosition` (`self.ArcGISLocation`) _returnvalue_3)
        (`KismetSystemLibrary.Delay` 0.5)
        (bind _returnvalue_4 (`ArcGISPoint.CreateArcGISPointWithXYZSpatialReference` -117.1825 34.055 0.0 _returnvalue_2))
        (`self.SetOrigin` _returnvalue_4)
        (bind _returnvalue_5 (`ArcGISPoint.GetX` _returnvalue))
        (bind _returnvalue_6 (`ArcGISPoint.GetY` _returnvalue))
        (`KismetSystemLibrary.PrintString` (`KismetStringLibrary.Concat_StrStr` (`KismetStringLibrary.Conv_DoubleToString` _returnvalue_5) ", " (`KismetStringLibrary.Conv_DoubleToString` _returnvalue_6))))
      (:`Is Not Valid`
        (`KismetSystemLibrary.PrintString` "Hello")))))

(fn `UserConstructionScript`)