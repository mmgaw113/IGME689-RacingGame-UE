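; bp_SplineMeshCreator places spline and spline mesh geometry on an ArcGIS map from X/Y coordinates.
; On BeginPlay it finds the ArcGISMapActor, whose MapComponent converts ArcGIS points to engine positions.
; Two events set and print the SplineMesh start and end positions from converted points.
; CreateSpline converts a geometry pair, then either inserts it as a world-space spline point or prints it, returning the position.
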(event `self.ReceiveBeginPlay`
  (bind _returnvalue (`GameplayStatics.GetActorOfClass` "/Script/ArcGISMapsSDK.ArcGISMapActor"))
  (set `self.MapComponent` _returnvalue))

(event `SetStartMeshPosition`
  (params (x :type "Float (double-precision)") (y :type "Float (double-precision)"))
  (bind _returnvalue (`ArcGISPoint.CreateArcGISPointWithXY` x y))
  (bind _returnvalue_2 (`ArcGISMapComponent.TransformPointToEnginePosition` (`ArcGISMapActor.MapComponent` (`self.MapComponent`)) _returnvalue))
  (`SplineMeshComponent.SetStartPosition` (`self.SplineMesh`) _returnvalue_2 true)
  (`KismetSystemLibrary.PrintString` (`KismetStringLibrary.Conv_VectorToString` _returnvalue_2)))

(event `SetEndPosition`
  (params (x :type "Float (double-precision)") (y :type "Float (double-precision)"))
  (bind _returnvalue (`ArcGISPoint.CreateArcGISPointWithXY` x y))
  (bind _returnvalue_2 (`ArcGISMapComponent.TransformPointToEnginePosition` (`ArcGISMapActor.MapComponent` (`self.MapComponent`)) _returnvalue))
  (`SplineMeshComponent.SetEndPosition` (`self.SplineMesh`) _returnvalue_2 true)
  (`KismetSystemLibrary.PrintString` (`KismetStringLibrary.Conv_VectorToString` _returnvalue_2)))

(fn `CreateSpline`
  (params (Index :type Integer) (Geometry :type "Geometries Structure") (AddToSpline :type Boolean))
  (returns (NewPosition :type "Vector Structure"))
  (bind _geometry (break `Geometries` Geometry))
  (bind _returnvalue (`ArcGISPoint.CreateArcGISPointWithXY` (`|GetArrayItem` _geometry) (`|GetArrayItem` _geometry 1)))
  (bind _returnvalue_2 (`ArcGISMapComponent.TransformPointToEnginePosition` (`ArcGISMapActor.MapComponent` (`self.MapComponent`)) _returnvalue))
  (if AddToSpline
    (`SplineComponent.AddSplinePointAtIndex` (`self.Spline`) _returnvalue_2 Index "World" true)
    (else
      (`KismetSystemLibrary.PrintString` (`KismetStringLibrary.Conv_VectorToString` _returnvalue_2))))
  (return _returnvalue_2))

(fn `UserConstructionScript`)